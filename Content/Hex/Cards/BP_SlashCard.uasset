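; BP_SlashCard is a hex-grid card that performs a slash across three neighboring tiles: the one in the chosen direction and the two flanking it.
; Activate calls the parent, resolves each tile index through the GameMode using adjacent-direction offsets, then activates each valid tile with 1 damage and the card's activation time.
; CanActivate requires only that the tile in the chosen direction is valid, ignoring the parent's result.
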(fn `Activate`
  (params (TileIdx :type Integer) (Dir :type "/Game/Hex/E_Dir Enum" :default "NewEnumerator0"))
  (bind _gamemode (`self.GameMode`))
  (bind _gamemode_2 (`self.GameMode`))
  (bind _gamemode_3 (`self.GameMode`))
  (`parent.Activate` TileIdx Dir)
  (`|ExecutionSequence`
    (:`then_0`
      (bind (_valid _idx) (`/Game/Hex/BP_TilingGameMode.GetValidIndexFromDir` _gamemode_2 Dir TileIdx))
      (if _valid
        (`/Game/Hex/BP_Hexpad.ActivateTile` (`|GetArrayItem` (`/Game/Hex/BP_TilingGameMode.Tiles` _gamemode_2) _idx) (`self.ActivationTime`) 1)))
    (:`then_1`
      (bind (_valid_2 _idx_2) (`/Game/Hex/BP_TilingGameMode.GetValidIndexFromDir` _gamemode_3 (`/Game/Hex/Helpers.GetAdjacentDir` 1 Dir) TileIdx))
      (if _valid_2
        (`/Game/Hex/BP_Hexpad.ActivateTile` (`|GetArrayItem` (`/Game/Hex/BP_TilingGameMode.Tiles` _gamemode_3) _idx_2) (`self.ActivationTime`) 1)))
    (:`then_2`
      (bind (_valid_3 _idx_3) (`/Game/Hex/BP_TilingGameMode.GetValidIndexFromDir` _gamemode (`/Game/Hex/Helpers.GetAdjacentDir` -1 Dir) TileIdx))
      (if _valid_3
        (`/Game/Hex/BP_Hexpad.ActivateTile` (`|GetArrayItem` (`/Game/Hex/BP_TilingGameMode.Tiles` _gamemode) _idx_3) (`self.ActivationTime`) 1)))))

(fn `CanActivate`
  (params (CurrentTileIdx :type Integer) (DIr :type "/Game/Hex/E_Dir Enum" :default "NewEnumerator0"))
  (returns (CanActivate :type Boolean))
  (`parent.CanActivate` CurrentTileIdx DIr)
  (bind _valid (`/Game/Hex/BP_TilingGameMode.GetValidIndexFromDir` (`self.GameMode`) DIr CurrentTileIdx))
  (return _valid))

(fn `UserConstructionScript`
  (`parent.UserConstructionScript`))