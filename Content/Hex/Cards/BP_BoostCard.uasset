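; Boost card for the hex game that dashes the player in a straight line across the tile grid.
; Activate steps through GameMode's valid-index lookup in the chosen direction until it is blocked or the distance counter reaches five, then sets the player's current tile index.
; CanActivate requires the next two tiles in that direction to be valid and movable.
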(fn `Activate`
  (params (TileIdx :type Integer) (Dir :type "/Game/Hex/E_Dir Enum" :default "NewEnumerator0"))
  (locals (Loop :type Boolean :default true) (NewIndex :type Integer) (DistanceCounter :type Integer))
  (`parent.Activate` TileIdx Dir)
  (set `local.NewIndex` TileIdx)
  (while (`local.Loop`)
    (bind (_valid _idx) (`/Game/Hex/BP_TilingGameMode.GetValidIndexFromDir` (`self.GameMode`) Dir (`local.NewIndex`)))
    (if _valid
      (set `local.NewIndex` _idx)
      (bind _result (`/Engine/EditorBlueprintResources/StandardMacros.IncrementInt` (`local.DistanceCounter`))
        (:`  `
          (if (>= _result 5)
            (set `local.Loop` false))))
      (else
        (set `local.Loop` false))))
  (bind _asbp_player (cast `/Game/Hex/BP_Player` (`GameplayStatics.GetPlayerPawn` 0)))
  (set `/Game/Hex/BP_Player.CurrentTileIndex` (`local.NewIndex`) _asbp_player))

(fn `CanActivate`
  (params (CurrentTileIdx :type Integer) (DIr :type "/Game/Hex/E_Dir Enum" :default "NewEnumerator0"))
  (returns (CanActivate :type Boolean))
  (bind _gamemode (`self.GameMode`))
  (bind _tiles (`/Game/Hex/BP_TilingGameMode.Tiles` _gamemode))
  (`parent.CanActivate` CurrentTileIdx DIr)
  (bind _idx (`/Game/Hex/BP_TilingGameMode.GetIndexFromDir` _gamemode DIr CurrentTileIdx))
  (bind _idx_2 (`/Game/Hex/BP_TilingGameMode.GetIndexFromDir` _gamemode DIr _idx))
  (bind _returnvalue (and (`/Game/Hex/BP_TilingGameMode.IsDirValid` _gamemode DIr CurrentTileIdx) (`/Game/Hex/BP_TilingGameMode.IsDirValid` _gamemode DIr _idx)))
  (if _returnvalue
    (return (and (`/Game/Hex/BP_Hexpad.CanMove` (`|GetArrayItem` _tiles _idx_2)) (`/Game/Hex/BP_Hexpad.CanMove` (`|GetArrayItem` _tiles _idx))))
    (else
      (return _returnvalue))))

(fn `UserConstructionScript`
  (`parent.UserConstructionScript`))