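; BP_BaseCard is the base card Blueprint for the hex tiling game, defining Activate, CanActivate, OnSelected and OnDeactivation hooks.
; Activate, CanActivate and OnSelected lazily cache the BP_TilingGameMode reference when it is not yet valid.
; The hooks carry no card behavior of their own: CanActivate returns false after caching, OnDeactivation is empty, and the event graph is unused.
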(fn `Activate`
  (params (TileIdx :type Integer) (Dir :type "/Game/Hex/E_Dir Enum" :default "NewEnumerator0"))
  (if (not (`KismetSystemLibrary.IsValid` (`self.GameMode`)))
    (bind _asbp_tiling_game_mode (cast `/Game/Hex/BP_TilingGameMode` (`GameplayStatics.GetGameMode`)))
    (set `self.GameMode` _asbp_tiling_game_mode)))

(fn `CanActivate`
  (params (CurrentTileIdx :type Integer) (DIr :type "/Game/Hex/E_Dir Enum" :default "NewEnumerator0"))
  (returns (CanActivate :type Boolean))
  (if (not (`KismetSystemLibrary.IsValid` (`self.GameMode`)))
    (bind _asbp_tiling_game_mode (cast `/Game/Hex/BP_TilingGameMode` (`GameplayStatics.GetGameMode`)))
    (set `self.GameMode` _asbp_tiling_game_mode)
    (return false)))

(fn `OnDeactivation`)

(fn `OnSelected`
  (if (not (`KismetSystemLibrary.IsValid` (`self.GameMode`)))
    (bind _asbp_tiling_game_mode (cast `/Game/Hex/BP_TilingGameMode` (`GameplayStatics.GetGameMode`)))
    (set `self.GameMode` _asbp_tiling_game_mode)))

(fn `UserConstructionScript`)