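; BP_WorldCard is a card Blueprint for a hex-tile game that works out which tiles can be selected around the player.
; On selection, it queries GetSelectableTilesFromDir for six directions from BP_Player's current tile and gathers the unique results into SelectableTiles, which deactivation clears.
; GetSelectableTilesFromDir is an empty stub here, so this class alone supplies no tiles.
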(fn `GetSelectableTiles`
  (returns (Tiles :type "Array of /Game/Hex/BP_Hexpad Object Reference"))
  (return (`self.SelectableTiles`)))

(fn `GetSelectableTilesFromDir`
  (params (Dir :type "/Game/Hex/E_Dir Enum" :default "NewEnumerator0") (CurrentTile :type Integer))
  (returns (Tiles :type "Array of /Game/Hex/BP_Hexpad Object Reference"))
  (return))

(fn `OnDeactivation`
  (`KismetArrayLibrary.Array_Clear` (`self.SelectableTiles`)))

(fn `OnSelected`
  (`parent.OnSelected`)
  (bind _asbp_player (cast `/Game/Hex/BP_Player` (`GameplayStatics.GetPlayerPawn` 0)))
  (for _index (range 6)
    (bind _tiles (`self.GetSelectableTilesFromDir` (cast `/Game/Hex/E_Dir` (`KismetMathLibrary.Conv_IntToByte` _index)) (`/Game/Hex/BP_TilePawn.CurrentTileIndex` _asbp_player)))
    (for _array_element _tiles
      (`KismetArrayLibrary.Array_AddUnique` (`self.SelectableTiles`) _array_element))))

(fn `UserConstructionScript`
  (`parent.UserConstructionScript`))