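; Player actor for a hex-tile board that steps between neighboring tiles held by BP_TilingGameMode.
; Six directional inputs or a mouse click, snapped to a hex direction by VecToDir, feed SetNextTile, which updates CurrentTileIndex for valid, walkable tiles.
; Tick interpolates the actor toward that tile and draws a debug arrow to the neighbor toward the hovered BP_Hexpad.
; MoveAmount resets on a debug Backspace but is never spent here.
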(event Input|EnhancedActionEvents|EnhancedInputActionIA_left
  (params (ActionValue :type Boolean) (ElapsedSeconds :type Float%20%28double-precision%29) (TriggeredSeconds :type Float%20%28double-precision%29) (InputAction :type Input%20Action%20Object%20Reference :default "/Game/Hex/input/IA_left.IA_left"))
  ;[0.15 0.15 0.15 0.5] numpad movement
  (bind _idx (Default|GetIndexfromDir (Variables|Default|GetGameModeRef) "NewEnumerator5" (Variables|Default|GetCurrentTileIndex)))
  (CallFunction|SetNextTile _idx "NewEnumerator5"))

(event Input|EnhancedActionEvents|EnhancedInputActionIA_Right
  (params (ActionValue :type Boolean) (ElapsedSeconds :type Float%20%28double-precision%29) (TriggeredSeconds :type Float%20%28double-precision%29) (InputAction :type Input%20Action%20Object%20Reference :default "/Game/Hex/input/IA_Right.IA_Right"))
  ;[0.15 0.15 0.15 0.5] numpad movement
  (bind _idx (Default|GetIndexfromDir (Variables|Default|GetGameModeRef) "NewEnumerator2" (Variables|Default|GetCurrentTileIndex)))
  (CallFunction|SetNextTile _idx "NewEnumerator2"))

(event Input|EnhancedActionEvents|EnhancedInputActionIA_UpLeft
  (params (ActionValue :type Boolean) (ElapsedSeconds :type Float%20%28double-precision%29) (TriggeredSeconds :type Float%20%28double-precision%29) (InputAction :type Input%20Action%20Object%20Reference :default "/Game/Hex/input/IA_UpLeft.IA_UpLeft"))
  ;[0.15 0.15 0.15 0.5] numpad movement
  (bind _idx (Default|GetIndexfromDir (Variables|Default|GetGameModeRef) "NewEnumerator0" (Variables|Default|GetCurrentTileIndex)))
  (CallFunction|SetNextTile _idx "NewEnumerator0"))

(event Input|EnhancedActionEvents|EnhancedInputActionIA_UpRight
  (params (ActionValue :type Boolean) (ElapsedSeconds :type Float%20%28double-precision%29) (TriggeredSeconds :type Float%20%28double-precision%29) (InputAction :type Input%20Action%20Object%20Reference :default "/Game/Hex/input/IA_UpRight.IA_UpRight"))
  ;[0.15 0.15 0.15 0.5] numpad movement
  (bind _idx (Default|GetIndexfromDir (Variables|Default|GetGameModeRef) "NewEnumerator1" (Variables|Default|GetCurrentTileIndex)))
  (CallFunction|SetNextTile _idx "NewEnumerator1"))

(event Input|EnhancedActionEvents|EnhancedInputActionIA_DownLeft
  (params (ActionValue :type Boolean) (ElapsedSeconds :type Float%20%28double-precision%29) (TriggeredSeconds :type Float%20%28double-precision%29) (InputAction :type Input%20Action%20Object%20Reference :default "/Game/Hex/input/IA_DownLeft.IA_DownLeft"))
  ;[0.15 0.15 0.15 0.5] numpad movement
  (bind _idx (Default|GetIndexfromDir (Variables|Default|GetGameModeRef) "NewEnumerator4" (Variables|Default|GetCurrentTileIndex)))
  (CallFunction|SetNextTile _idx "NewEnumerator4"))

(event Input|EnhancedActionEvents|EnhancedInputActionIA_DownRight
  (params (ActionValue :type Boolean) (ElapsedSeconds :type Float%20%28double-precision%29) (TriggeredSeconds :type Float%20%28double-precision%29) (InputAction :type Input%20Action%20Object%20Reference :default "/Game/Hex/input/IA_DownRight.IA_DownRight"))
  ;[0.15 0.15 0.15 0.5] numpad movement
  (bind _idx (Default|GetIndexfromDir (Variables|Default|GetGameModeRef) "NewEnumerator3" (Variables|Default|GetCurrentTileIndex)))
  (CallFunction|SetNextTile _idx "NewEnumerator3"))

(event Input|EnhancedActionEvents|EnhancedInputActionIA_Click
  (params (ActionValue :type Boolean) (ElapsedSeconds :type Float%20%28double-precision%29) (TriggeredSeconds :type Float%20%28double-precision%29) (InputAction :type Input%20Action%20Object%20Reference :default "/Game/Hex/input/IA_Click.IA_Click"))
  (bind _returnvalue (Transformation|GetActorLocation))
  (if (< (Class|KismetMathLibrary|VectorDistanceSquared (Transformation|GetActorLocation) (CallFunction|GetTilePos (Variables|Default|GetCurrentTileIndex))) 1e+02)
    (bind _returnvalue_2 (Class|WidgetLayoutLibrary|GetMousePositiononViewport))
    (bind _outhit (Collision|LineTraceByChannel (.WorldPosition (Class|GameplayStatics|DeprojectScreentoWorld (Game|GetPlayerController 0) _returnvalue_2)) (+ (* (.WorldDirection (Class|GameplayStatics|DeprojectScreentoWorld (Game|GetPlayerController 0) _returnvalue_2)) 10000) (.WorldPosition (Class|GameplayStatics|DeprojectScreentoWorld (Game|GetPlayerController 0) _returnvalue_2))) "TraceTypeQuery1" false 0 "None"))
    (bind _asbp_hexpad (Utilities|Casting|CastToBP_Hexpad (.hitactor _outhit)))
    (bind _dir (CallFunction|VectoDir (- (Math|Vector|MakeVector (.x (Transformation|GetActorLocation _asbp_hexpad)) (.y (Transformation|GetActorLocation _asbp_hexpad)) 0.0) (Math|Vector|MakeVector (.x _returnvalue) (.y _returnvalue) 0.0))))
    (bind _idx (Default|GetIndexfromDir (Variables|Default|GetGameModeRef) _dir (Variables|Default|GetCurrentTileIndex)))
    (CallFunction|SetNextTile _idx _dir)))

(event EventBeginPlay
  (bind _asbp_tiling_game_mode (Utilities|Casting|CastToBP_TilingGameMode (Game|GetGameMode)))
  (Variables|Default|SetGameModeRef _asbp_tiling_game_mode)
  (Transformation|SetActorLocation (CallFunction|GetTilePos (Variables|Default|GetCurrentTileIndex)) false false)
  (Variables|Default|SetMoveAmount (Variables|Default|GetMaxMoveAmount)))

(event Collision|EventActorBeginOverlap
  (params (OtherActor :type Actor%20Object%20Reference)))

(event EventTick
  (params (DeltaSeconds :type Float%20%28single-precision%29))
  (bind _returnvalue (Transformation|GetActorLocation))
  (bind _currenttileindex (Variables|Default|GetCurrentTileIndex))
  (bind _tilepos (CallFunction|GetTilePos _currenttileindex))
  (Utilities|FlowControl|Sequence
    (:then_0
      ;[0.15 0.15 0.15 0.5] movement
      (Transformation|SetActorLocation (Math|Interpolation|VInterpTo (Transformation|GetActorLocation) (CallFunction|GetTilePos (Variables|Default|GetCurrentTileIndex)) DeltaSeconds 8.0) false false))
    (:then_1
      ;[0.15 0.15 0.15 0.5] Draw arrow
      (bind _returnvalue_2 (Class|WidgetLayoutLibrary|GetMousePositiononViewport))
      (bind _outhit (Collision|LineTraceByChannel (.WorldPosition (Class|GameplayStatics|DeprojectScreentoWorld (Game|GetPlayerController 0) _returnvalue_2)) (+ (* (.WorldDirection (Class|GameplayStatics|DeprojectScreentoWorld (Game|GetPlayerController 0) _returnvalue_2)) 10000) (.WorldPosition (Class|GameplayStatics|DeprojectScreentoWorld (Game|GetPlayerController 0) _returnvalue_2))) "TraceTypeQuery1" false 0 "None"))
      (bind _asbp_hexpad (Utilities|Casting|CastToBP_Hexpad (.hitactor _outhit)))
      (bind _dir (CallFunction|VectoDir (- (Math|Vector|MakeVector (.x (Transformation|GetActorLocation _asbp_hexpad)) (.y (Transformation|GetActorLocation _asbp_hexpad)) 0.0) (Math|Vector|MakeVector (.x _returnvalue) (.y _returnvalue) 0.0))))
      (bind _idx (Default|GetIndexfromDir (Variables|Default|GetGameModeRef) _dir _currenttileindex))
      (if (< (Class|KismetMathLibrary|DistanceSquared2D (Math|Vector2D|MakeVector2D (.x _tilepos) (.y _tilepos)) (Math|Vector2D|MakeVector2D (.x (CallFunction|GetTilePos _idx)) (.y (CallFunction|GetTilePos _idx)))) 5e+04)
        (Rendering|Debug|DrawDebugArrow (Math|Vector|MakeVector (.x _tilepos) (.y _tilepos) 5e+01) (Math|Vector|MakeVector (.x (CallFunction|GetTilePos _idx)) (.y (CallFunction|GetTilePos _idx)) 5e+01) 8e+01 "(R=0.344253,G=1.000000,B=0.340278,A=1.000000)" 0.0 1e+01)))))

(event Input|KeyboardEvents|DebugKeyBackspace
  (params (Key :type Key%20Structure :default "None") (ActionValue :type Input%20Action%20Value%20Structure))
  ;[0.15 0.15 0.15 0.5] next round
  (:Pressed
    (Variables|Default|SetMoveAmount (Variables|Default|GetMaxMoveAmount))))

(fn ConstructionScript)

(fn GetTilePos
  (params (idx :type Integer))
  (return (Transformation|GetActorLocation (Utilities|Array|Get(acopy) (Variables|/Game/Hex/BP_TilingGameMode.BP_TilingGameMode_C|GetTiles (Variables|Default|GetGameModeRef)) idx))))

(fn SetNextTile
  (params (id :type Integer) (Dir :type E_Dir%20Enum :default "NewEnumerator0"))
  (bind _gamemoderef (Variables|Default|GetGameModeRef))
  (if (Default|IsDirValid _gamemoderef Dir (Variables|Default|GetCurrentTileIndex))
    (if (Variables|/Game/Hex/BP_Hexpad.BP_Hexpad_C|GetCanMove (Utilities|Array|Get(acopy) (Variables|/Game/Hex/BP_TilingGameMode.BP_TilingGameMode_C|GetTiles _gamemoderef) id))
      (Variables|Default|SetCurrentTileIndex id))))

(fn VectoDir
  (params (VectorDir :type Vector))
  (bind _returnvalue (Math|Vector|Normalize VectorDir 0.001))
  (if (> (.y _returnvalue) 0.0)
    (if (> (.x _returnvalue) 0.0)
      (if (> (.x _returnvalue) 0.433)
        (return "NewEnumerator1")
        (else
          _))
      (elif (> (.x _returnvalue) -0.433)
        _
        (else
          (return "NewEnumerator3"))))
    (return "NewEnumerator2")
    (else
      (if (> (.x _returnvalue) 0.0)
        (if (> (.x _returnvalue) 0.433)
          (return "NewEnumerator0")
          (else
            _))
        (elif (> (.x _returnvalue) -0.433)
          _
          (else
            (return "NewEnumerator4"))))
      (return "NewEnumerator5"))))