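; Game mode that builds a hexagonal tile board at BeginPlay and adds the player's input mapping context.
; It spawns indexed BP_Hexpad actors row by row, alternating each row's sideways offset via 60-degree trigonometry, and stores them in Tiles.
; GetIndexFromDir finds a neighbour index in six directions using row parity.
; GetValidIndexFromDir pairs that index with IsDirValid, a stub that always returns false.
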(event `self.ReceiveBeginPlay`
  (`EnhancedInputSubsystemInterface.AddMappingContext` (pcsubsystem `EnhancedInputLocalPlayerSubsystem` (`GameplayStatics.GetPlayerController` 0)) "/Game/Hex/input/IMC_Player.IMC_Player" 0 (struct))
  (for _index (range (* (`self.TileRows`) (`self.TileCols`)))
    (bind _returnvalue (mod _index (`self.TileCols`)))
    (if (and (== _returnvalue 0) (!= _index 0))
      (set `self.LineSpawnPos` (+ (`KismetMathLibrary.MakeVector` (* (`KismetMathLibrary.DegSin` 60.0) (`self.DistBetweenTiles`)) (* (`KismetMathLibrary.DegCos` 60.0) (* (`self.Coloffset`) (`self.DistBetweenTiles`)))) (`self.LineSpawnPos`)))
      (if (== (`self.Coloffset`) 1)
        (set `self.Coloffset` -1)
        (else
          (set `self.Coloffset` 1))))
    (bind _returnvalue_2 (`|SpawnActorFromClass` "/Game/Hex/BP_Hexpad.BP_Hexpad_C" (`KismetMathLibrary.MakeTransform` (+ (`KismetMathLibrary.MakeVector` 0.0 (* _returnvalue (`self.DistBetweenTiles`))) (`self.LineSpawnPos`))) "Undefined" "MultiplyWithRoot" null null))
    (set `/Game/Hex/BP_Hexpad.index` _index _returnvalue_2)
    (`KismetArrayLibrary.Array_Add` (`self.Tiles`) _returnvalue_2)))

(fn `GetIndexFromDir`
  (params (Dir :type "/Game/Hex/E_Dir Enum" :default "NewEnumerator0") (CurrentIndex :type Integer))
  (returns (Idx :type Integer))
  (bind _tilecols (`self.TileCols`))
  (bind _returnvalue (`KismetMathLibrary.SelectInt` 1 0 (== (mod (`KismetMathLibrary.FFloor` (/ (`KismetMathLibrary.Conv_IntToDouble` CurrentIndex) (`self.TileCols`))) 2) 0)))
  (return (select `/Game/Hex/E_Dir` Dir :`NewEnumerator0` (+ CurrentIndex (- _tilecols _returnvalue)) :`NewEnumerator1` (+ CurrentIndex (- _tilecols -1 _returnvalue)) :`NewEnumerator2` (+ CurrentIndex 1) :`NewEnumerator3` (- CurrentIndex (+ _tilecols -1 _returnvalue)) :`NewEnumerator4` (- CurrentIndex (+ _tilecols _returnvalue)) :`NewEnumerator5` (- CurrentIndex 1))))

(fn `GetValidIndexFromDir`
  (params (Dir :type "/Game/Hex/E_Dir Enum" :default "NewEnumerator0") (`Current Index` :type Integer))
  (returns (valid :type Boolean) (Idx :type Integer))
  (bind _idx (`self.GetIndexFromDir` Dir `Current Index`))
  (bind _newparam (`self.IsDirValid` Dir))
  (return _newparam _idx))

(fn `IsDirValid`
  (params (Dir :type "/Game/Hex/E_Dir Enum" :default "NewEnumerator0"))
  (returns (NewParam :type Boolean))
  (return false))

(fn `UserConstructionScript`)