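; BP_Hexpad is a hex tile actor that is either movable or blocked and can be temporarily lit as activated.
; The construction script randomly blocks roughly one in ten tiles, clearing CanMove and applying the blocked material.
; ActivateTile gives movable tiles the activated material and a cooldown duration.
; Tick counts that cooldown down and restores the default tile material when it drops below zero.
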(event `self.ReceiveBeginPlay`)

(event `self.ReceiveTick`
  (params (DeltaSeconds :type "Float (single-precision)"))
  (bind _activationcooldown (`self.ActivationCooldown`))
  (if (> _activationcooldown 0.0)
    (bind _output_get (set `self.ActivationCooldown` (- _activationcooldown DeltaSeconds)))
    (if (< _output_get 0.0)
      (`PrimitiveComponent.SetMaterial` (`self.HexTile`) 0 "/Game/Hex/M_Tile.M_Tile"))))

(fn `ActivateTile`
  (params (Time :type "Float (double-precision)"))
  (if (`self.CanMove`)
    (set `self.ActivationCooldown` Time)
    (`PrimitiveComponent.SetMaterial` (`self.HexTile`) 0 "/Game/Hex/M_ActivatedTile.M_ActivatedTile")))

(fn `UserConstructionScript`
  (if (> (`KismetMathLibrary.RandomInteger` 100) 90)
    (set `self.CanMove` false)
    (`PrimitiveComponent.SetMaterial` (`self.HexTile`) 0 "/Game/Hex/M_BlockedTile.M_BlockedTile")))